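; Boss actor for a space shooter, damaged by overlaps from "Bullet"-tagged actors on two hit components, with explosions at the wing sockets.
; A DoOnce with short delay throttles HP loss; death spawns GC_Squitd_Blueprint, notifies Space_gameMode and destroys the actor.
; A looping timer targets a player-proximity check that creates the boss HP bar widget, with no guard against duplicates.
; BeginPlay also collects four arrows as movement points, unused here.
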(event `self.ReceiveBeginPlay`
  (bind _movementpoints (`self.MovementPoints`))
  (`|ExecutionSequence`
    (:`then_0`
      (bind _asspace_game_mode (cast `Space_gameMode` (`GameplayStatics.GetGameMode`)))
      (set `self.GM_reff` _asspace_game_mode))
    (:`then_1`
      (`KismetArrayLibrary.Array_Add` _movementpoints (`self.Arrow`))
      (`KismetArrayLibrary.Array_Add` _movementpoints (`self.Arrow1`))
      (`KismetArrayLibrary.Array_Add` _movementpoints (`self.Arrow2`))
      (`KismetArrayLibrary.Array_Add` _movementpoints (`self.Arrow3`)))
    (:`then_2`
      (set `self.HP` (`self.MAxHP`))
      (`KismetSystemLibrary.K2_SetTimer` null "Near player UI" 0.5 true))))

(event `self.hit.OnComponentBeginOverlap`
  (params (OverlappedComponent :type "PrimitiveComponent Object Reference") (OtherActor :type "Actor Object Reference") (OtherComp :type "PrimitiveComponent Object Reference") (OtherBodyIndex :type Integer) (bFromSweep :type Boolean) (SweepResult :type "HitResult Structure (by ref)"))
  (if (`self.ActorHasTag` OtherActor "Bullet")
    (`GameplayStatics.SpawnEmitterAtLocation` "/Game/StarterContent/Particles/P_Explosion.P_Explosion" (`SceneComponent.GetSocketLocation` (`self.hit`) "WingL") (struct) (2.0 2.0 2.0) true "AutoRelease")
    (`self.Damage` :!label _label)))

(event `self.hit1.OnComponentBeginOverlap`
  (params (OverlappedComponent :type "PrimitiveComponent Object Reference") (OtherActor :type "Actor Object Reference") (OtherComp :type "PrimitiveComponent Object Reference") (OtherBodyIndex :type Integer) (bFromSweep :type Boolean) (SweepResult :type "HitResult Structure (by ref)"))
  (if (`self.ActorHasTag` OtherActor "Bullet")
    (`GameplayStatics.SpawnEmitterAtLocation` "/Game/StarterContent/Particles/P_Explosion.P_Explosion" (`SceneComponent.GetSocketLocation` (`self.hit1`) "WingR") (struct) (2.0 2.0 2.0) true "AutoRelease")
    (goto _label)))

(event `Damage`
  (`|ExecutionSequence`
    (:`then_0`
      (`/Engine/EditorBlueprintResources/StandardMacros.DoOnce` false :!label _label_2
        (:`Completed`
          (bind _result (`/Engine/EditorBlueprintResources/StandardMacros.DecrementFloat` (`self.HP`))
            (:`  `
              (set `self.HP` _result)
              (`KismetSystemLibrary.Delay` 0.2)
              (goto _label_2 :!via `Reset`))))))
    (:`then_1`
      (if (< (`self.HP`) 0.0)
        (`self.Death`)))))

(event `Near player UI`
  (bind _returnvalue_x (`KismetMathLibrary.BreakVector` (`SceneComponent.K2_GetComponentLocation` (`self.Root`))))
  (bind _returnvalue_x_2 (`KismetMathLibrary.BreakVector` (`SceneComponent.K2_GetComponentLocation` (`Actor.RootComponent` (`self.PlayerRef`)))))
  (`KismetSystemLibrary.Delay` 1.0)
  (if (< (- _returnvalue_x _returnvalue_x_2) 8000.0)
    (bind _returnvalue (`|CreateWidget` "/Game/Boss/Boss1/BP_bossHP_bar1.BP_bossHP_bar1_C"))
    (`UserWidget.AddToViewport` _returnvalue 0)))

(event `Death`
  (bind _returnvalue (`KismetMathLibrary.RandomFloatInRange` -35.0 45.0))
  (`KismetSystemLibrary.Delay` 1.0)
  (`|SpawnActorFromClass` "/Game/Enemys/Model_Explosion/GC_Squitd_Blueprint.GC_Squitd_Blueprint_C" (`KismetMathLibrary.MakeTransform` (`SceneComponent.K2_GetComponentLocation` (`self.BossMesh`)) (`KismetMathLibrary.MakeRotator` 90.0 _returnvalue _returnvalue)) "Undefined" "MultiplyWithRoot" null null)
  (`Space_gameMode.OnBossDefeated` (`self.GM_reff`))
  (`self.K2_DestroyActor`))

(fn `UserConstructionScript`)