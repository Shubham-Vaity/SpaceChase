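; BP_space_dirag is a space-level boss that loses HP to "Bullet"-tagged overlaps and reports its defeat to BP_Space_gameMode.
; Each hit spawns an explosion and costs one HP, throttled by a resetting DoOnce.
; A looping timer targets a player X-distance check that adds a boss HP bar widget.
; Death spawns GC_Squitd_Blueprint, increments player BossKills and destroys the boss; movement points are collected but unused here.
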(event `self.ReceiveBeginPlay`
  (bind _movementpoints (`self.MovementPoints`))
  (`|ExecutionSequence`
    (:`then_0`
      (bind _asbp_space_game_mode (cast `/Game/test/BP_Space_gameMode` (`GameplayStatics.GetGameMode`)))
      (set `self.GM_reff` _asbp_space_game_mode))
    (:`then_1`
      (set `self.HP` (`self.MAxHP`))
      (`KismetSystemLibrary.K2_SetTimer` null "Near player UI" 0.5 true))
    (:`then_2`
      (`KismetArrayLibrary.Array_Add` _movementpoints)
      (`KismetArrayLibrary.Array_Add` _movementpoints (`self.Arrow2`))
      (`KismetArrayLibrary.Array_Add` _movementpoints (`self.Arrow3`))
      (`KismetArrayLibrary.Array_Add` _movementpoints (`self.Arrow1`)))
    (:`then_3`
      (bind _asbp_playable_player (cast `/Game/test/BP_PlayablePlayer` (`GameplayStatics.GetPlayerCharacter` 0)))
      (set `self.Player_reff` _asbp_playable_player))))

(event `self.Box.OnComponentBeginOverlap`
  (params (OverlappedComponent :type "PrimitiveComponent Object Reference") (OtherActor :type "Actor Object Reference") (OtherComp :type "PrimitiveComponent Object Reference") (OtherBodyIndex :type Integer) (bFromSweep :type Boolean) (SweepResult :type "HitResult Structure (by ref)"))
  (if (`self.ActorHasTag` OtherActor "Bullet")
    (`GameplayStatics.SpawnEmitterAtLocation` "/Game/StarterContent/Particles/P_Explosion.P_Explosion" (`SceneComponent.K2_GetComponentLocation` (`self.BossMesh`)) (struct) (2.0 2.0 2.0) true "AutoRelease")
    (`self.Damage`)))

(event `Damage`
  (`|ExecutionSequence`
    (:`then_0`
      (`/Engine/EditorBlueprintResources/StandardMacros.DoOnce` false :!label _label
        (:`Completed`
          (bind _result (`/Engine/EditorBlueprintResources/StandardMacros.DecrementFloat` (`self.HP`))
            (:`  `
              (set `self.HP` _result)
              (`KismetSystemLibrary.Delay` 0.2)
              (goto _label :!via `Reset`))))))
    (:`then_1`
      (if (< (`self.HP`) 0.0)
        (`self.Death`)))))

(event `Near player UI`
  (bind _returnvalue_x (`KismetMathLibrary.BreakVector` (`SceneComponent.K2_GetComponentLocation` (`self.Root`))))
  (bind _returnvalue_x_2 (`KismetMathLibrary.BreakVector` (`SceneComponent.K2_GetComponentLocation` (`Actor.RootComponent` (`self.Player_reff`)))))
  (`KismetSystemLibrary.Delay` 1.0)
  (if (< (- _returnvalue_x _returnvalue_x_2) 8000.0)
    (bind _returnvalue (`|CreateWidget` "/Game/Boss/Boss7/BP_bossHP_bar6.BP_bossHP_bar6_C"))
    (`UserWidget.AddToViewport` _returnvalue 0)))

(event `Death`
  (bind _returnvalue (`KismetMathLibrary.RandomFloatInRange` -35.0 45.0))
  (bind _player_reff (`self.Player_reff`))
  (`/Engine/EditorBlueprintResources/StandardMacros.DoOnce` false
    (:`Completed`
      (set `Space_gameMode.BossActive` false (`self.GM_reff`))
      (`|ExecutionSequence`
        (:`then_0`
          (`KismetSystemLibrary.Delay` 1.0)
          (`|SpawnActorFromClass` "/Game/Enemys/Model_Explosion/GC_Squitd_Blueprint.GC_Squitd_Blueprint_C" (`KismetMathLibrary.MakeTransform` (`SceneComponent.K2_GetComponentLocation` (`self.BossMesh`)) (`KismetMathLibrary.MakeRotator` 90.0 _returnvalue _returnvalue)) "Undefined" "MultiplyWithRoot" null null)
          (`Space_gameMode.OnBossDefeated` (`self.GM_reff`))
          (`self.K2_DestroyActor`))
        (:`then_1`
          (bind _result (`/Game/EditorBlueprintResources/StandardMacros.IncrementInt` (`/Game/test/BP_PlayablePlayer.Boss_kills` _player_reff))
            (:`  `
              (set `/Game/test/BP_PlayablePlayer.Boss_kills` _result _player_reff))))))))

(fn `UserConstructionScript`)