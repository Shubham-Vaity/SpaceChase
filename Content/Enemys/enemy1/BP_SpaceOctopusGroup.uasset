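; BP_SpaceOctopusGroup is an enemy actor that flies one of four preset movement patterns, then destroys itself.
; GetPattern takes a position index and plays the matching timeline, whose Y and Z tracks drive a swept SetActorLocation while X stays at the root's value.
; Two of the patterns first rotate the skeletal mesh 180 degrees.
; The index is also printed for debugging, immediately and after a short delay.
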(event `self.GetPattern`
  (params (Possition :type Integer))
  (bind _returnvalue_x (`KismetMathLibrary.BreakVector` (`SceneComponent.K2_GetComponentLocation` (`self.DefaultSceneRoot`))))
  (bind _returnvalue_x_2 (`KismetMathLibrary.BreakVector` (`SceneComponent.K2_GetComponentLocation` (`self.DefaultSceneRoot`))))
  (bind _returnvalue_x_3 (`KismetMathLibrary.BreakVector` (`SceneComponent.K2_GetComponentLocation` (`self.DefaultSceneRoot`))))
  (bind _returnvalue_x_4 (`KismetMathLibrary.BreakVector` (`SceneComponent.K2_GetComponentLocation` (`self.DefaultSceneRoot`))))
  (`|ExecutionSequence`
    (:`then_0`
      (`KismetSystemLibrary.PrintString` (`KismetStringLibrary.Conv_IntToString` Possition))
      (if (== Possition 0)
        (bind (_direction _y _z) (`Timeline|Timeline_2`)
          (:`Update`
            (`self.K2_SetActorLocation` (`KismetMathLibrary.MakeVector` _returnvalue_x _y _z) true))
          (:`Finished`
            (`self.K2_DestroyActor`)))
        (elif (== Possition 1)
          (`SceneComponent.K2_SetWorldRotation` (`self.SkeletalMesh`) (struct :`Yaw` 180.0) false false)
          (bind (_direction_2 _y_2 _z_2) (`Timeline|Timeline`)
            (:`Update`
              (`self.K2_SetActorLocation` (`KismetMathLibrary.MakeVector` _returnvalue_x_2 _y_2 _z_2) true))
            (:`Finished`
              (`self.K2_DestroyActor`)))
          (elif (== Possition 2)
            (`SceneComponent.K2_SetWorldRotation` (`self.SkeletalMesh`) (struct :`Yaw` 180.0) false false)
            (bind (_direction_3 _y_3 _z_3) (`Timeline|Timeline_0`)
              (:`Update`
                (`self.K2_SetActorLocation` (`KismetMathLibrary.MakeVector` _returnvalue_x_3 _y_3 _z_3) true))
              (:`Finished`
                (`self.K2_DestroyActor`)))
            (else
              (bind (_direction_4 _y_4 _z_4) (`Timeline|Timeline_1`)
                (:`Update`
                  (`self.K2_SetActorLocation` (`KismetMathLibrary.MakeVector` _returnvalue_x_4 _y_4 _z_4) true))
                (:`Finished`
                  (`self.K2_DestroyActor`))))))))
    (:`then_1`
      (`KismetSystemLibrary.Delay` 1.0)
      (`KismetSystemLibrary.PrintString` (`KismetStringLibrary.Conv_IntToString` Possition)))))

(fn `UserConstructionScript`)