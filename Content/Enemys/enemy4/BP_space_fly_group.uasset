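; BP_space_fly_group is a flying enemy that follows one of four preset paths and can be shot down by the player.
; GetPattern selects a Timeline that sweeps it through Y/Z at fixed X, flips the mesh for two patterns, reveals it after a brief delay and destroys it at path end.
; A Bullet-tagged HitBox overlap spawns GC_Fish_Blueprint oriented by pattern, increments player Kills, plays a death sound and destroys the actor.
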(event `self.ReceiveBeginPlay`
  (bind _asbp_playable_player (cast `/Game/test/BP_PlayablePlayer` (`GameplayStatics.GetPlayerCharacter` 0)))
  (set `self.Player_reff` _asbp_playable_player))

(event `self.GetPattern`
  (params (Possition :type Integer))
  (bind _returnvalue_x (`KismetMathLibrary.BreakVector` (`self.K2_GetActorLocation`)))
  (bind _returnvalue_x_2 (`KismetMathLibrary.BreakVector` (`self.K2_GetActorLocation`)))
  (bind _returnvalue_x_3 (`KismetMathLibrary.BreakVector` (`self.K2_GetActorLocation`)))
  (bind _returnvalue_x_4 (`KismetMathLibrary.BreakVector` (`self.K2_GetActorLocation`)))
  (`|ExecutionSequence`
    (:`then_0`
      (if (== Possition 0)
        (bind (_direction _y _z) (`Timeline|Timeline_2`)
          (:`Update`
            (`self.K2_SetActorLocation` (`KismetMathLibrary.MakeVector` _returnvalue_x _y _z) true))
          (:`Finished`
            (`self.K2_DestroyActor`)))
        (elif (== Possition 1)
          (`SceneComponent.K2_SetWorldRotation` (`self.SkeletalMesh`) (struct :`Yaw` 180.0) false false)
          (bind (_direction_2 _y_2 _z_2) (`Timeline|Timeline`)
            (:`Update`
              (`self.K2_SetActorLocation` (`KismetMathLibrary.MakeVector` _returnvalue_x_2 _y_2 _z_2) true))
            (:`Finished`
              (`self.K2_DestroyActor`)))
          (elif (== Possition 2)
            (`SceneComponent.K2_SetWorldRotation` (`self.SkeletalMesh`) (struct :`Yaw` 180.0) false false)
            (bind (_direction_3 _y_3 _z_3) (`Timeline|Timeline_0`)
              (:`Update`
                (`self.K2_SetActorLocation` (`KismetMathLibrary.MakeVector` _returnvalue_x_3 _y_3 _z_3) true))
              (:`Finished`
                (`self.K2_DestroyActor`)))
            (else
              (bind (_direction_4 _y_4 _z_4) (`Timeline|Timeline_1`)
                (:`Update`
                  (`self.K2_SetActorLocation` (`KismetMathLibrary.MakeVector` _returnvalue_x_4 _y_4 _z_4) true))
                (:`Finished`
                  (`self.K2_DestroyActor`))))))))
    (:`then_1`
      (set `self.Possition` Possition)
      (`KismetSystemLibrary.Delay` 0.1)
      (`SceneComponent.SetVisibility` (`self.SkeletalMesh`) true false))))

(event `self.hitBox.OnComponentBeginOverlap`
  (params (OverlappedComponent :type "PrimitiveComponent Object Reference") (OtherActor :type "Actor Object Reference") (OtherComp :type "PrimitiveComponent Object Reference") (OtherBodyIndex :type Integer) (bFromSweep :type Boolean) (SweepResult :type "HitResult Structure (by ref)"))
  (bind _player_reff (`self.Player_reff`))
  (bind _possition (`self.Possition`))
  (if (`self.ActorHasTag` OtherActor "Bullet")
    (if (or (== _possition 1) (== _possition 2))
      (`|SpawnActorFromClass` "/Game/Enemys/Model_Explosion/GC_Fish_Blueprint.GC_Fish_Blueprint_C" (`KismetMathLibrary.MakeTransform` (+ (`SceneComponent.K2_GetComponentLocation` (`self.SkeletalMesh`)) (1000.0 0.0 0.0))) "Undefined" "MultiplyWithRoot" null null)
      (else
        (`|SpawnActorFromClass` "/Game/Enemys/Model_Explosion/GC_Fish_Blueprint.GC_Fish_Blueprint_C" (`KismetMathLibrary.MakeTransform` (+ (`SceneComponent.K2_GetComponentLocation` (`self.SkeletalMesh`)) (1000.0 0.0 0.0)) (struct :`Yaw` 180.0)) "Undefined" "MultiplyWithRoot" null null)))
    (bind _result (`/Engine/EditorBlueprintResources/StandardMacros.IncrementInt` (`/Game/test/BP_PlayablePlayer.Kills` _player_reff))
      (:`  `
        (set `/Game/test/BP_PlayablePlayer.Kills` _result _player_reff)
        (`GameplayStatics.SpawnSound2D` "/Game/music/death.death" 1.0 1.0 0.0 null)
        (`self.K2_DestroyActor`)))))

(fn `UserConstructionScript`)