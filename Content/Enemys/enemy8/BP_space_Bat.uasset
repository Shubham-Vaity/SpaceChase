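; BP_space_Bat is an enemy that dies in one hit from anything tagged "Bullet".
; On BeginPlay it caches a reference to the BP_PlayablePlayer character.
; A bullet overlapping its HitBox spawns GC_Squitd_Blueprint at the mesh location with semi-random rotation, increments the player's Kills and destroys the bat.
; No movement or attack logic is defined in this Blueprint.
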(event `self.ReceiveBeginPlay`
  (bind _asbp_playable_player (cast `/Game/test/BP_PlayablePlayer` (`GameplayStatics.GetPlayerCharacter` 0)))
  (set `self.Player_reff` _asbp_playable_player))

(event `self.hitBox.OnComponentBeginOverlap`
  (params (OverlappedComponent :type "PrimitiveComponent Object Reference") (OtherActor :type "Actor Object Reference") (OtherComp :type "PrimitiveComponent Object Reference") (OtherBodyIndex :type Integer) (bFromSweep :type Boolean) (SweepResult :type "HitResult Structure (by ref)"))
  (bind _returnvalue (`KismetMathLibrary.RandomFloatInRange` -35.0 45.0))
  (bind _player_reff (`self.Player_reff`))
  (bind _kills (`/Game/test/BP_PlayablePlayer.Kills` _player_reff))
  (if (`self.ActorHasTag` OtherActor "Bullet")
    (`|SpawnActorFromClass` "/Game/Enemys/Model_Explosion/GC_Squitd_Blueprint.GC_Squitd_Blueprint_C" (`KismetMathLibrary.MakeTransform` (`SceneComponent.K2_GetComponentLocation` (`self.SkeletalMesh`)) (`KismetMathLibrary.MakeRotator` 90.0 _returnvalue _returnvalue)) "Undefined" "MultiplyWithRoot" null null)
    (`/Engine/EditorBlueprintResources/StandardMacros.IncrementInt` _kills
      (:`  `
        (set `/Game/test/BP_PlayablePlayer.Kills` _kills _player_reff)
        (`self.K2_DestroyActor`)))))

(fn `UserConstructionScript`)