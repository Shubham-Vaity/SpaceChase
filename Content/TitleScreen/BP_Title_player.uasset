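; BP_Title_player is the title screen player whose camera reacts to hover on the play, options, credits, controls and quit entries.
; Each hover event plays its own timeline forward, or reverses it when hover ends.
; Play slides the camera along world X, options and quit pitch it, and credits and controls yaw it, with each rotation zeroing the other axes.
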(event `Playe`
  (params (hover :type Boolean))
  (bind _camera (`self.Camera`))
  (bind (_returnvalue_x _returnvalue_y _returnvalue_z) (`KismetMathLibrary.BreakVector` (`SceneComponent.K2_GetComponentLocation` _camera)))
  (if hover
    (bind (_direction _x) (`Timeline|play` :!label _label)
      (:`Update`
        (`SceneComponent.K2_SetWorldLocation` _camera (`KismetMathLibrary.MakeVector` _x _returnvalue_y _returnvalue_z) false false)))
    (else
      (goto _label :!via `Reverse`))))

(event `Options`
  (params (hover :type Boolean))
  (if hover
    (bind (_direction _y) (`Timeline|opt` :!label _label_2)
      (:`Update`
        (`SceneComponent.K2_SetRelativeRotation` (`self.Camera`) (`KismetMathLibrary.MakeRotator` 0.0 _y) false false)))
    (else
      (goto _label_2 :!via `Reverse`))))

(event `creadites`
  (params (hov :type Boolean))
  (if hov
    (bind (_direction _x) (`Timeline|Crd` :!label _label_3)
      (:`Update`
        (`SceneComponent.K2_SetRelativeRotation` (`self.Camera`) (`KismetMathLibrary.MakeRotator` 0.0 0.0 _x) false false)))
    (else
      (goto _label_3 :!via `Reverse`))))

(event `controles`
  (params (hov :type Boolean))
  (if hov
    (bind (_direction _x) (`Timeline|Timeline` :!label _label_4)
      (:`Update`
        (`SceneComponent.K2_SetRelativeRotation` (`self.Camera`) (`KismetMathLibrary.MakeRotator` 0.0 0.0 _x) false false)))
    (else
      (goto _label_4 :!via `Reverse`))))

(event `quit`
  (params (hov :type Boolean))
  (if hov
    (bind (_direction _x) (`Timeline|Timeline_0` :!label _label_5)
      (:`Update`
        (`SceneComponent.K2_SetRelativeRotation` (`self.Camera`) (`KismetMathLibrary.MakeRotator` 0.0 _x) false false)))
    (else
      (goto _label_5 :!via `Reverse`))))

(fn `UserConstructionScript`)