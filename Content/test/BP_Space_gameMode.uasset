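; Space game mode that runs background music and the boss health bar.
; BeginPlay plays the main intro into a loop and starts a one-second timer polling BossActive.
; The Music event switches to boss intro and loop when active, then fades back to the main loop.
; BossBar adds a health widget while BossAlive; otherwise it creates and removes a new widget, leaving any existing bar untouched.
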(event `self.ReceiveBeginPlay`
  (`|ExecutionSequence`
    (:`then_0`
      (`GameplayStatics.PlaySound2D` "/Game/music/MP3_MIan_intro.MP3_MIan_intro" 1.0 1.0 0.0 null null)
      (`KismetSystemLibrary.Delay` 9.67)
      (bind _returnvalue (`GameplayStatics.SpawnSound2D` "/Game/music/MP3_Main_loop.MP3_Main_loop" 1.0 1.0 0.0 null))
      (set `self.MainLoop` _returnvalue))
    (:`then_1`
      (`KismetSystemLibrary.K2_SetTimer` null "Music" 1.0 true))))

(event `Music`
  (bind _boss (`self.boss`))
  (if (`self.BossActive`)
    (if (`self.MusicPlay`)
      (set `self.MusicPlay` false)
      (`AudioComponent.FadeOut` (`self.MainLoop`) 0.5 0.0 "Linear")
      (`GameplayStatics.SpawnSound2D` "/Game/music/MP3_Boss_intro.MP3_Boss_intro" 1.0 1.0 0.0 null)
      (`KismetSystemLibrary.Delay` 12.878)
      (bind _returnvalue (`GameplayStatics.SpawnSound2D` "/Game/music/MP3_Boss_loop.MP3_Boss_loop" 1.0 1.0 0.0 null))
      (set `self.boss` _returnvalue))
    (else
      (`/Game/EditorBlueprintResources/StandardMacros.IsValid` _boss
        (:`Is Valid`
          (`AudioComponent.FadeOut` _boss 0.5 0.0 "Linear")
          (bind _returnvalue_2 (`GameplayStatics.SpawnSound2D` "/Game/music/MP3_Main_loop.MP3_Main_loop" 1.0 1.0 0.0 null))
          (set `self.MainLoop` _returnvalue_2)
          (set `self.MusicPlay` true))))))

(event `BossBar`
  (if (`self.bBossAlive`)
    (bind _returnvalue (`|CreateWidget` "/Game/Boss/BP_bossHP_bar.BP_bossHP_bar_C"))
    (`UserWidget.AddToViewport` _returnvalue 0)
    (else
      (bind _returnvalue_2 (`|CreateWidget` "/Game/Boss/BP_bossHP_bar.BP_bossHP_bar_C"))
      (`Widget.RemoveFromParent` _returnvalue_2))))

(fn `UserConstructionScript`)