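; Test enemy actor that uses homing projectile movement, then switches to a scripted movement pattern once it exactly reaches the player.
; BeginPlay caches the player, assigns the homing target component and starts a looping timer intended to poll the player capsule's location.
; When the enemy's root matches that location, homing turns off and the Move timeline plays.
; The timeline offsets the enemy from the captured location with sweeping moves and sets a negative initial projectile speed.
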(event `self.ReceiveBeginPlay`
  (`|ExecutionSequence`
    (:`then_0`
      (bind _asmy_playable_player (cast `/Game/test/MyPlayablePlayer` (`GameplayStatics.GetPlayerCharacter` 0)))
      (set `self.PlayerReff` _asmy_playable_player)
      (`KismetSystemLibrary.K2_SetTimer` null "Get location" 0.1 true))
    (:`then_1`
      (set `ProjectileMovementComponent.HomingTargetComponent` (`self.Homing Target Component`) (`self.ProjectileMovement`)))))

(event `Get location`
  (bind _output_get (set `self.location` (`SceneComponent.K2_GetComponentLocation` (`Character.CapsuleComponent` (`self.PlayerReff`)))))
  (if (== (`SceneComponent.K2_GetComponentLocation` (`self.DefaultSceneRoot`)) _output_get)
    (set `ProjectileMovementComponent.bIsHomingProjectile` false (`self.ProjectileMovement`))
    (`self.pattern`)))

(event `pattern`
  (bind (_location_x _location_y _location_z) (`KismetMathLibrary.BreakVector` (`self.location`)))
  (bind (_direction _y _z) (`Timeline|move`)
    (:`Update`
      (`SceneComponent.K2_SetWorldLocation` (`self.DefaultSceneRoot`) (`KismetMathLibrary.MakeVector` (+ _location_x 500.0) (+ _y _location_y) (+ _z _location_z)) true false)
      (set `ProjectileMovementComponent.InitialSpeed` -400.0 (`self.ProjectileMovement`)))))

(fn `UserConstructionScript`)