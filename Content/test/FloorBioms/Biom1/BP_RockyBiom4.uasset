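; BP_RockyBiom4 is a rocky biome floor piece, judging by its name and folder, that registers four spawn points.
; On BeginPlay it adds its four Arrow components to the SpawnArrows array, with no parent BeginPlay call in the graph.
; The construction script only calls the parent version, and nothing in this Blueprint reads the array or spawns from it.
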(event `self.ReceiveBeginPlay`
  (bind _spawnarrows (`self.SpawnArrows`))
  (`KismetArrayLibrary.Array_Add` _spawnarrows (`self.Arrow`))
  (`KismetArrayLibrary.Array_Add` _spawnarrows (`self.Arrow1`))
  (`KismetArrayLibrary.Array_Add` _spawnarrows (`self.Arrow2`))
  (`KismetArrayLibrary.Array_Add` _spawnarrows (`self.Arrow3`)))

(fn `UserConstructionScript`
  (`parent.UserConstructionScript`))