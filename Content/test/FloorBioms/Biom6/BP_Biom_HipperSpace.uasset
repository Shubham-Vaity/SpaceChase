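; HipperSpace floor biome Blueprint that supplies its own set of spawn arrows to logic inherited from a parent class.
; On BeginPlay it runs the parent logic, then appends four entries, including its Arrow components, to the SpawnArrows array.
; The construction script only calls the parent, and Tick and overlap events are disabled, so this file adds no other behavior.
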(event `self.ReceiveBeginPlay`
  (bind _spawnarrows (`self.SpawnArrows`))
  (`parent.ReceiveBeginPlay`)
  (`KismetArrayLibrary.Array_Add` _spawnarrows)
  (`KismetArrayLibrary.Array_Add` _spawnarrows (`self.Arrow2`))
  (`KismetArrayLibrary.Array_Add` _spawnarrows (`self.Arrow`))
  (`KismetArrayLibrary.Array_Add` _spawnarrows (`self.Arrow1`)))

(fn `UserConstructionScript`
  (`parent.UserConstructionScript`))